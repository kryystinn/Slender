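; Note is a collectible pickup actor that the first-person player character can collect by interacting with it.
; A Box component's overlap events set an IsOverlaping flag while a FirstPersonCharacter is inside it.
; The Interact event, when that flag is set, destroys the note and increments the NumNotes counter on player 0's FirstPersonCharacter.
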(event `/Game/NPCs/Gatekeeper/Interact.Interact`
  (if (`self.isOverlaping`)
    (`self.K2_DestroyActor`)
    (bind _asfirst_person_character (cast `/Game/FirstPersonBP/Blueprints/FirstPersonCharacter` (`GameplayStatics.GetPlayerCharacter` 0)))
    (set `/Game/FirstPersonBP/Blueprints/FirstPersonCharacter.NumNotes` (+ (`/Game/FirstPersonBP/Blueprints/FirstPersonCharacter.NumNotes` _asfirst_person_character) 1) _asfirst_person_character)))

(event `self.Box.OnComponentBeginOverlap`
  (params (OverlappedComponent :type "PrimitiveComponent Object Reference") (OtherActor :type "Actor Object Reference") (OtherComp :type "PrimitiveComponent Object Reference") (OtherBodyIndex :type Integer) (bFromSweep :type Boolean) (SweepResult :type "HitResult Structure (by ref)"))
  (cast `/Game/FirstPersonBP/Blueprints/FirstPersonCharacter` OtherActor)
  (set `self.isOverlaping` true))

(event `self.Box.OnComponentEndOverlap`
  (params (OverlappedComponent :type "PrimitiveComponent Object Reference") (OtherActor :type "Actor Object Reference") (OtherComp :type "PrimitiveComponent Object Reference") (OtherBodyIndex :type Integer))
  (cast `/Game/FirstPersonBP/Blueprints/FirstPersonCharacter` OtherActor)
  (set `self.isOverlaping` false))

(fn `UserConstructionScript`)