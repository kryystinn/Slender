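; An interactable rock that the first-person player can shift aside once.
; A box overlap tracks whether the player is in range and shows a text prompt until the rock has moved.
; Interact, while in range, instantly offsets the actor horizontally, sets a Moved flag and hides the prompt.
; A Tick gate, opened on first valid overlap and never closed, keeps the text rotated toward the player.
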(event `self.ReceiveBeginPlay`
  (`SceneComponent.SetVisibility` (`self.TextRender`) false false))

(event `/Game/NPCs/Gatekeeper/Interact.Interact`
  (if (`self.isOverlaping`)
    (if (not (`self.moved`))
      (`self.K2_SetActorLocation` (+ (`self.K2_GetActorLocation`) (-500.0 -500.0 0.0)))
      (set `self.moved` true)
      (`SceneComponent.SetVisibility` (`self.TextRender`) false false))))

(event `self.ReceiveTick`
  (params (DeltaSeconds :type "Float (single-precision)"))
  (`/Engine/EditorBlueprintResources/StandardMacros.Gate` true :!label _label
    (:`Exit`
      (`SceneComponent.K2_SetWorldRotation` (`self.TextRender`) (`KismetMathLibrary.FindLookAtRotation` (`self.K2_GetActorLocation`) (`self.K2_GetActorLocation` (`GameplayStatics.GetPlayerCharacter` 0))) false false))))

(event `self.Box.OnComponentBeginOverlap`
  (params (OverlappedComponent :type "PrimitiveComponent Object Reference") (OtherActor :type "Actor Object Reference") (OtherComp :type "PrimitiveComponent Object Reference") (OtherBodyIndex :type Integer) (bFromSweep :type Boolean) (SweepResult :type "HitResult Structure (by ref)"))
  (cast `/Game/FirstPersonBP/Blueprints/FirstPersonCharacter` OtherActor)
  (set `self.isOverlaping` true)
  (if (not (`self.moved`))
    (`SceneComponent.SetVisibility` (`self.TextRender`) true false)
    (goto _label :!via `Open`)))

(event `self.Box.OnComponentEndOverlap`
  (params (OverlappedComponent :type "PrimitiveComponent Object Reference") (OtherActor :type "Actor Object Reference") (OtherComp :type "PrimitiveComponent Object Reference") (OtherBodyIndex :type Integer))
  (cast `/Game/FirstPersonBP/Blueprints/FirstPersonCharacter` OtherActor)
  (set `self.isOverlaping` false)
  (`SceneComponent.SetVisibility` (`self.TextRender`) false false))

(fn `UserConstructionScript`)