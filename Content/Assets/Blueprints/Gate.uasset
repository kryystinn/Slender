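; Gate actor that the player removes by interacting with it, provided the first-person character's OpenGate flag is set.
; The Interact event reads that flag from player 0's FirstPersonCharacter and destroys the gate when true.
; A box overlap shows and hides a text render, hidden at BeginPlay.
; Any overlapping actor toggles the text, as the character cast on begin overlap runs after the visibility change.
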(event `self.ReceiveBeginPlay`
  (`SceneComponent.SetVisibility` (`self.TextRender`) false false))

(event `/Game/NPCs/Gatekeeper/Interact.Interact`
  (bind _asfirst_person_character (cast `/Game/FirstPersonBP/Blueprints/FirstPersonCharacter` (`GameplayStatics.GetPlayerCharacter` 0)))
  (if (`/Game/FirstPersonBP/Blueprints/FirstPersonCharacter.openGate` _asfirst_person_character)
    (`self.K2_DestroyActor`)))

(event `self.Box.OnComponentBeginOverlap`
  (params (OverlappedComponent :type "PrimitiveComponent Object Reference") (OtherActor :type "Actor Object Reference") (OtherComp :type "PrimitiveComponent Object Reference") (OtherBodyIndex :type Integer) (bFromSweep :type Boolean) (SweepResult :type "HitResult Structure (by ref)"))
  (`SceneComponent.SetVisibility` (`self.TextRender`) true false)
  (cast `/Game/FirstPersonBP/Blueprints/FirstPersonCharacter` OtherActor))

(event `self.Box.OnComponentEndOverlap`
  (params (OverlappedComponent :type "PrimitiveComponent Object Reference") (OtherActor :type "Actor Object Reference") (OtherComp :type "PrimitiveComponent Object Reference") (OtherBodyIndex :type Integer))
  (`SceneComponent.SetVisibility` (`self.TextRender`) false false))

(fn `UserConstructionScript`)